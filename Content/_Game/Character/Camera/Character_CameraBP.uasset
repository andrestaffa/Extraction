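; Player camera manager for the FPS character that drives the first-person view while a weapon is equipped, except during vaulting or climbing.
; BlueprintUpdateCamera blends from the player camera toward a point derived from the weapon's IronSight socket by ADSValue, narrowing FOV alongside.
; Tick interpolates a sway offset from turn and look input, with separate ADS and idle variants, which is rotated into view space and added to camera location.
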(event Custom|CE_WeaponSway
  (Utilities|IsValid (Variables|Default|GetPlayer)
    (:Is%20Valid
      (Variables|Default|SetSwayOffset (Math|Interpolation|VInterpTo (Variables|Default|GetSwayOffset) "0, 0, 0" (Utilities|Time|GetWorldDeltaSeconds) 8.0))
      (Variables|Default|SetSwayOffset (Math|Interpolation|VInterpTo (Variables|Default|GetSwayOffset) (select (Variables|/Script/Extraction.FPSCharacter|GetADSEnabled (Variables|Default|GetPlayer)) (Utilities|SwayADS) (Utilities|SwayIndle)) (Utilities|Time|GetWorldDeltaSeconds) 5.0)))))

(event EventTick
  (params (DeltaSeconds :type Float%20%28single-precision%29))
  (CallFunction|CEWeaponSway))

(fn ConstructionScript)

(fn BlueprintUpdateCamera
  (params (CameraTarget :type Actor%20Object%20Reference))
  (bind _asbp_fpscharacter (Utilities|Casting|CastToBP_FPSCharacter CameraTarget))
  (bind _output_get (Variables|Default|SetPlayer _asbp_fpscharacter))
  (Utilities|IsValid _output_get
    (:Is%20Valid
      (if (not (or (Variables|/Script/Extraction.FPSCharacter|GetisVaulting (Variables|Default|GetPlayer)) (Variables|/Script/Extraction.FPSCharacter|GetisClimbing (Variables|Default|GetPlayer))))
        (Utilities|IsValid (Variables|/Script/Extraction.FPSCharacter|GetequippedWeapon (Variables|Default|GetPlayer))
          (:Is%20Valid
            (Variables|Default|SetFinalCameraRotation (Pawn|GetControlRotation (Variables|Default|GetPlayer) :!class /Script/Engine.Pawn))
            (Variables|Default|SetFinalCameraLocation (+ (Math|Vector|Lerp(Vector) (Transformation|GetWorldLocation (Variables|/Game/_Game/Character/BP_FPSCharacter.BP_FPSCharacter_C|GetPlayerCamera (Variables|Default|GetPlayer))) (- (.Location (Math|Transform|BreakTransform (Transformation|GetSocketTransform (Variables|/Script/Extraction.Item|GetitemMesh (Variables|/Script/Extraction.FPSCharacter|GetequippedWeapon (Variables|Default|GetPlayer))) "IronSight" "RTS_World"))) (* (Math|Vector|GetForwardVector (.Rotation (Math|Transform|BreakTransform (Transformation|GetSocketTransform (Variables|/Script/Extraction.Item|GetitemMesh (Variables|/Script/Extraction.FPSCharacter|GetequippedWeapon (Variables|Default|GetPlayer))) "IronSight" "RTS_World")))) (* (Math|Vector|DotProduct (Math|Vector|Normalize (- (.Location (Math|Transform|BreakTransform (Transformation|GetSocketTransform (Variables|/Script/Extraction.Item|GetitemMesh (Variables|/Script/Extraction.FPSCharacter|GetequippedWeapon (Variables|Default|GetPlayer))) "IronSight" "RTS_World"))) (Transformation|GetWorldLocation (Variables|/Game/_Game/Character/BP_FPSCharacter.BP_FPSCharacter_C|GetPlayerCamera (Variables|Default|GetPlayer)))) 0.0) (Math|Vector|GetForwardVector (.Rotation (Math|Transform|BreakTransform (Transformation|GetSocketTransform (Variables|/Script/Extraction.Item|GetitemMesh (Variables|/Script/Extraction.FPSCharacter|GetequippedWeapon (Variables|Default|GetPlayer))) "IronSight" "RTS_World"))))) (/ (Math|Vector|VectorLength (- (.Location (Math|Transform|BreakTransform (Transformation|GetSocketTransform (Variables|/Script/Extraction.Item|GetitemMesh (Variables|/Script/Extraction.FPSCharacter|GetequippedWeapon (Variables|Default|GetPlayer))) "IronSight" "RTS_World"))) (Transformation|GetWorldLocation (Variables|/Game/_Game/Character/BP_FPSCharacter.BP_FPSCharacter_C|GetPlayerCamera (Variables|Default|GetPlayer))))) 2.5e+02)))) (Variables|/Script/Extraction.FPSCharacter|GetADSValue (Variables|Default|GetPlayer))) (Math|Vector|RotateVector (Variables|Default|GetSwayOffset) (Variables|Default|GetFinalCameraRotation))))
            (return (Variables|Default|GetFinalCameraLocation) (Variables|Default|GetFinalCameraRotation) (Math|Float|Lerp 9e+01 8e+01 (Variables|/Script/Extraction.FPSCharacter|GetADSValue (Variables|Default|GetPlayer))) true)))))))